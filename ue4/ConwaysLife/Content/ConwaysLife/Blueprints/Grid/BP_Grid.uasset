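; BP_Grid is the grid actor for Conway's Life, drawing a width-by-height field of cells as hierarchical instanced static meshes.
; Generate stores the dimensions, clears old instances and adds one per cell, spaced by cell size plus gap and using the root's world location and scale.
; It then shifts the HISM component by half the total extent to center the grid.
; BeginPlay, the width and height update events, and the construction script are empty.
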(event Custom|UpdateWidth
  (params (newWidth :type Integer)))

(event Custom|UpdateHeight
  (params (newHeight :type Integer)))

(event EventBeginPlay)

(fn ConstructionScript)

(fn Generate
  (params (w :type Integer) (h :type Integer))
  (bind _defaultsceneroot (Variables|Default|GetDefaultSceneRoot))
  (bind _returnvalue (Transformation|GetWorldLocation _defaultsceneroot))
  (bind (_x _y _z) (Math|Vector|BreakVector _returnvalue))
  (bind _output_get (Variables|Default|Setwidth w))
  (bind _output_get_2 (Variables|Default|Setheigth h))
  (Components|InstancedStaticMesh|ClearInstances (Variables|Default|GetHISM_Grid))
  (for _index (range 0 (- _output_get_2 1))
    (for _index_2 (range 0 (- _output_get 1))
      (Components|InstancedStaticMesh|AddInstance (Variables|Default|GetHISM_Grid) (Math|Transform|MakeTransform (Math|Vector|MakeVector (+ (* _index_2 (Math|Conversions|ToFloat(Integer) (+ (Variables|Default|Getcell_width) (Variables|Default|Getbetween)))) _x) (+ (* _index (Math|Conversions|ToFloat(Integer) (+ (Variables|Default|Getcell_height) (Variables|Default|Getbetween)))) _y) _z) "0, 0, 0" (Transformation|GetWorldScale _defaultsceneroot)))))
  (bind _output_get_3 (Variables|Default|Setfull_width (Math|Conversions|ToFloat(Integer) (* (Variables|Default|Getwidth) (+ (Variables|Default|Getcell_width) (Variables|Default|Getbetween))))))
  (bind _output_get_4 (Variables|Default|Setfull_height (Math|Conversions|ToFloat(Integer) (* (Variables|Default|Getheigth) (+ (Variables|Default|Getcell_height) (Variables|Default|Getbetween))))))
  (Transformation|SetRelativeLocation (Variables|Default|GetHISM_Grid) (Math|Vector|MakeVector (/ _output_get_3 -2.0) (/ _output_get_4 -2.0) 0.0) false true))